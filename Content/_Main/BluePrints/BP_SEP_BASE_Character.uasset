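; Base character Blueprint that sets up team-aware proximity voice chat and a mic level meter.
; On BeginPlay it creates the meter widget and adds a VOIPTalker, retrying until PlayerState is valid before registering it.
; TeamTag selects the talker's attenuation asset, attached to the first-person camera, and its OnRep copies it into actor Tags.
; An audio envelope handler maps levels to MicValue, but its binding node never runs.
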(event `self.ReceiveBeginPlay`
  ; Initialize and Start Voice chat
  (`WidgetBlueprintLibrary.SetInputMode_GameOnly` (`GameplayStatics.GetPlayerController` 0))
  (`self.Initialize Voice Chat`)
  ;; Create Mic Level UI
  (bind _returnvalue (`|CreateWidget` "/Game/VoiceChat/WB_MicMeter.WB_MicMeter_C"))
  (`UserWidget.AddToViewport` _returnvalue 0))

(event `Initialize Voice Chat`
  (bind _playerstate (`self.PlayerState`))
  (bind _voip_ref (`self.VOIP REF`))
  ; Initialize and Start Voice chat
  (bind _returnvalue (`AddComponent|NODE_AddVOIPTalker-0`))
  (set `self.VOIP REF` _returnvalue)
  (`/Engine/EditorBlueprintResources/StandardMacros.IsValid` _playerstate :!label _label
    (:`Is Valid`
      (`VOIPTalker.RegisterWithPlayerState` (`self.VOIP REF`) _playerstate)
      (`VOIPStatics.SetMicThreshold` -1.0)
      (if (== (`self.TeamTag`) "Team resistance")
        (set `VOIPTalker.Settings` (make `VoiceSettings` (`self.FirstPersonCameraComponent`) "/Game/VoiceChat/SA_VOIP.SA_VOIP") _voip_ref)
        (else
          (set `VOIPTalker.Settings` (make `VoiceSettings` (`self.FirstPersonCameraComponent`) "/Game/VoiceChat/SA_Nazi.SA_Nazi") _voip_ref))))
    (:`Is Not Valid`
      (`KismetSystemLibrary.Delay` 0.2)
      (goto _label))))

(event `On Audio Envelope Value`
  (params (EnvelopeValue :type "Float (single-precision)"))
  ; Mic Audio Level to Float
  (set `self.MicValue` (`KismetMathLibrary.MapRangeClamped` (`KismetMathLibrary.Log` EnvelopeValue) -2.7 -0.7 0.0 1.0)))

(fn `OnRep_TeamTag`
  (`KismetArrayLibrary.Array_Set` (`self.Tags`) 0 (`self.TeamTag`) true))

(fn `UserConstructionScript`)