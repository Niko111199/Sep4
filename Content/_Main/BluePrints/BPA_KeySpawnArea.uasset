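; BPA_KeySpawnArea is a placeable volume that spawns keys and chests at random points inside its Box component.
; SpawnKeys, which its comment says GameMode calls for replication, spawns a single BPA_Key, then clears CanSpawn to block repeats.
; SpawnChest spawns a BPA_Chest the same way, with a small negative Y offset and no repeat guard.
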(event `Spawn Keys`
  (bind _box (`self.Box`))
  ;[1 0 0 0.5] Event to Spawn Keys, is called from GameMode, to Replicate
  (if (`self.Can spawn`)
    (`|SpawnActorFromClass` "/Game/_Main/BluePrints/BPA_Key.BPA_Key_C" (`KismetMathLibrary.Conv_VectorToTransform` (`KismetMathLibrary.RandomPointInBoundingBox` (`SceneComponent.K2_GetComponentLocation` _box) (`BoxComponent.GetScaledBoxExtent` _box))) "Undefined" "MultiplyWithRoot" null null)
    (set `self.Can spawn` false)))

(event `Spawn Chest`
  (bind _box (`self.Box`))
  ;[0 0.01742 0.15 0.5] Spawn Chest Random Place
  (`|SpawnActorFromClass` "/Game/_Main/BluePrints/BPA_Chest.BPA_Chest_C" (`KismetMathLibrary.Conv_VectorToTransform` (- (`KismetMathLibrary.RandomPointInBoundingBox` (`SceneComponent.K2_GetComponentLocation` _box) (`BoxComponent.GetScaledBoxExtent` _box)) (0.0 2.5 0.0))) "Undefined" "MultiplyWithRoot" null null))

(fn `UserConstructionScript`)