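; Door actor that lets Resistance characters open it from outside the prison, then closes itself.
; On BeginPlay the Door component is yawed open, and a separate CloseDoorOnBeginPlay event, not called here, resets the actor's rotation.
; A Trigger overlap plays the OpenDoor timeline to drive absolute actor yaw, with CloseDoor starting from its Update after a delay.
; CanOpen blocks retriggering until CloseDoor begins updating.
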(event `CloseDoorOnBeginPlay`
  ;[0.15 0.1125 0 0.5] Closes Door On Begin Play
  (`self.K2_SetActorRotation` (`KismetMathLibrary.MakeRotator` 0.0 0.0 180.0)))

(event `self.ReceiveBeginPlay`
  ;[0 0.0364 0.15 0.5] Set Door Rotation To Open At begin Play, so playes, cant be stuck in loppy play
  (`SceneComponent.K2_SetRelativeRotation` (`self.door`) (`KismetMathLibrary.MakeRotator` 0.0 0.0 -90.0) false false))

(event `self.Trigger.OnComponentBeginOverlap`
  (params (OverlappedComponent :type "PrimitiveComponent Object Reference") (OtherActor :type "Actor Object Reference") (OtherComp :type "PrimitiveComponent Object Reference") (OtherBodyIndex :type Integer) (bFromSweep :type Boolean) (SweepResult :type "HitResult Structure (by ref)"))
  ;[0 0.15 0.001302 0.5] Lets Resistance Players Open Door, to prison from Outside
  (if (`self.Can Open'`)
    (cast `/Game/_Main/BluePrints/BP_SEP_RessistanceBase_charactor` OtherActor)
    (bind (_direction _opendoor) (`Timeline|OpenDoor` :!via `PlayFromStart`)
      (:`Update`
        (`self.K2_SetActorRotation` (`KismetMathLibrary.MakeRotator` 0.0 0.0 _opendoor))
        (set `self.Can Open'` false)
        (`KismetSystemLibrary.Delay` 5.0)
        (bind (_direction_2 _closedoor) (`Timeline|CloseDoor` :!via `PlayFromStart`)
          (:`Update`
            (`self.K2_SetActorRotation` (`KismetMathLibrary.MakeRotator` 0.0 0.0 _closedoor))
            (set `self.Can Open'` true)))))))

(fn `UserConstructionScript`)