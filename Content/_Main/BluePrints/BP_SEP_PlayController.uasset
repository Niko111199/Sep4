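; Player controller that shows the team selection screen and requests team-based spawning for its player.
; On BeginPlay, the local controller creates WBP_TeamSelection and adds it to the viewport, only in the MainMap level.
; Its SpawnPlayer event passes a team tag and itself to BP_Sep_GameMode, which handles the actual spawn.
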(event `self.ReceiveBeginPlay`
  ;[0 0.15 0.0807 0.5] Spawn Team Widget
  (if (`self.IsLocalPlayerController`)
    (bind _returnvalue (`GameplayStatics.GetCurrentLevelName` true))
    (if (`KismetStringLibrary.EqualEqual_StrStr` _returnvalue "MainMap")
      (bind _returnvalue_2 (`|CreateWidget` "/Game/_Main/TeamSystem/WBP_TeamSelection.WBP_TeamSelection_C"))
      (`UserWidget.AddToViewport` _returnvalue_2 0))))

(event `SpawnPlayer`
  (params (TeamTag :type Name))
  ;[0.15 0.135 0 0.5] Calls Event To Spawn Players Diffrent Places Based On Team
  (bind _asbp_sep_game_mode (cast `/Game/_Main/BluePrints/BP_Sep_GameMode` (`GameplayStatics.GetGameMode`)))
  (`/Game/_Main/BluePrints/BP_Sep_GameMode.Spawn Player` _asbp_sep_game_mode TeamTag self))

(fn `UserConstructionScript`)