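; Game state for a two-sided multiplayer match, tracking found keys and ending the game with a Nazi or Resistance win.
; FindKey increments a RepNotify key count, updating key widgets directly on the server's first player controller and through OnRep on clients.
; Tick declares a Nazi win when RemainingTime runs out, while ChestOpen declares a Resistance win.
; Either outcome shows the win/lose widget and pauses the game.
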(event `self.ReceiveTick`
  (params (DeltaSeconds :type "Float (single-precision)"))
  ;[0 0.1276 0.15 0.5] Tick Events
  (`self.TimeWinCondition`))

(event `FindKey`
  ;[1 0.7877 0 0.5] Event To Find Key
  (`/Engine/EditorBlueprintResources/StandardMacros.IncrementInt` (`self.Number Of Keys Found`)
    (:`  `
      ;; Only Informs Server, Clients Is Informed by Repnotifyer
      (bind _asbp_sep_play_controller (cast `/Game/_Main/BluePrints/BP_SEP_PlayController` (`GameplayStatics.GetPlayerController` 0))
        (:`then`
          (`/Game/_Main/BluePrints/BP_SEP_PlayController.UpdateKeyWidgets` _asbp_sep_play_controller))
        (:`CastFailed`
          (`KismetSystemLibrary.PrintString` "failed to update server on key Info"))))))

(event `TimeWinCondition`
  ;[0 0.15 0.003476 0.5] Win Condition
  ;;[0 0.02315 0.15 0.5] Time Out
  (if (<= (`self.RemainingTime`) 0)
    (bind _returnvalue (`|CreateWidget` "/Game/_Main/BluePrints/BPW_WinLoseUI.BPW_WinLoseUI_C"))
    (`/Game/_Main/BluePrints/BPW_WinLoseUI.Set Nazi Win` _returnvalue)
    (`UserWidget.AddToViewport` _returnvalue 0)
    (`GameplayStatics.SetGamePaused` true)))

(event `ChestOpen`
  ;[0 0.15 0.003476 0.5] Win Condition
  ;;[0.9557 0.7527 0 0.5] Chest Opened
  (bind _returnvalue (`|CreateWidget` "/Game/_Main/BluePrints/BPW_WinLoseUI.BPW_WinLoseUI_C"))
  (`/Game/_Main/BluePrints/BPW_WinLoseUI.Set Resistance Win` _returnvalue)
  (`UserWidget.AddToViewport` _returnvalue 0)
  (`GameplayStatics.SetGamePaused` true))

(fn `OnRep_Number Of Keys Found`
  ; BroadCasts to Clients
  (bind _asbp_sep_play_controller (cast `/Game/_Main/BluePrints/BP_SEP_PlayController` (`GameplayStatics.GetPlayerController` 0))
    (:`then`
      (`/Game/_Main/BluePrints/BP_SEP_PlayController.UpdateKeyWidgets` _asbp_sep_play_controller))
    (:`CastFailed`
      (`KismetSystemLibrary.PrintText` "Failed to broeadcast Key Info"))))

(fn `UserConstructionScript`)