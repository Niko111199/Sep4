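; Game mode for a team-based match that gives the host a start-game button on BeginPlay.
; StartGame spawns keys through the key spawn area, starts a one-second countdown on the game state's remaining time, then loops over players.
; Each loop pass respawns that player, closes the door and starts all AI controllers.
; SpawnPlayer spawns and possesses a pawn at a random PlayerStart matching the team tag, then tags it.
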(event `Add Start Game Button to Host`
  ;[0.15 0 0.1209 0.5] Add Button To Start Game To Host Player
  (bind _returnvalue (`|CreateWidget` "/Game/_Main/BluePrints/WBP_HostStartGame.WBP_HostStartGame_C"))
  (`UserWidget.AddToViewport` _returnvalue 0))

(event `self.ReceiveBeginPlay`
  ;[0.04285 1 0 0.5] Calls Everthing in Begin
  (`self.Add Start Game Button to Host`))

(event `Spawn Player`
  (params (TeamTag :type Name) (PlayerController :type "/Game/_Main/BluePrints/BP_SEP_PlayController Object Reference") (Class :type "/Game/_Main/BluePrints/BP_SEP_BASE_Character Class Reference"))
  ;[0.02573 0 0.487 0.5] Event To Spawn Players of diffrent Team At diffrent spawn Points and set teamTag
  (bind _outactors (`GameplayStatics.GetAllActorsOfClassWithTag` "/Script/Engine.PlayerStart" TeamTag))
  (bind _returnvalue (`|SpawnActorFromClass` Class (`self.GetTransform` (`KismetArrayLibrary.Array_Random` _outactors)) "Undefined" "MultiplyWithRoot" null "None" null))
  (`Controller.Possess` PlayerController _returnvalue)
  (set `/Game/_Main/BluePrints/BP_SEP_BASE_Character.TeamTag` TeamTag _returnvalue))

(event `Spawn Keys In Map`
  ;[0 0.02626 0.15 0.5] Spawn Keys In Map
  (bind _outactors (`GameplayStatics.GetAllActorsOfClass` "/Game/_Main/BluePrints/BPA_KeySpawnArea.BPA_KeySpawnArea_C"))
  (`/Game/_Main/BluePrints/BPA_KeySpawnArea.Spawn Keys` (`|GetArrayItem` _outactors)))

(event `Start countdown`
  ; timer
  (`KismetSystemLibrary.K2_SetTimerDelegate` (delegate `CountdownEvent`) 1.0 true))

(event `CountdownEvent`
  ; timer
  (bind _asbp_sep_gamestate (cast `/Game/_Main/BluePrints/BP_SEP_Gamestate` (`GameplayStatics.GetGameState`)))
  (set `/Game/_Main/BluePrints/BP_SEP_Gamestate.RemainingTime` (`KismetMathLibrary.Clamp` (- (`/Game/_Main/BluePrints/BP_SEP_Gamestate.RemainingTime` _asbp_sep_gamestate) 1) 0 1000) _asbp_sep_gamestate))

(event `Start Game`
  ;[0 0.15 0.1423 0.5] Called By Host Player, to Start Game'
  (`self.Spawn Keys In Map`)
  (`self.Start countdown`)
  (for _array_element (`GameStateBase.PlayerArray` (`GameplayStatics.GetGameState`))
    (bind _asbp_sep_play_controller (cast `/Game/_Main/BluePrints/BP_SEP_PlayController` (`PlayerState.GetPlayerController` _array_element)))
    (`/Game/_Main/BluePrints/BP_SEP_PlayController.Respawn Player` _asbp_sep_play_controller)
    (bind _returnvalue (`GameplayStatics.GetActorOfClass` "/Game/_Main/BluePrints/BPA_Door.BPA_Door_C"))
    (`/Game/_Main/BluePrints/BPA_Door.CloseDoorOnBeginPlay` _returnvalue)
    (bind _outactors (`GameplayStatics.GetAllActorsOfClass` "/Game/_Main/AI/BP_SEP_AIController.BP_SEP_AIController_C"))
    (for _array_element_2 _outactors
      (`/Game/_Main/AI/BP_SEP_AIController.Start AI` _array_element_2))))

(fn `UserConstructionScript`)